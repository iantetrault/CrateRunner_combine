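; A spiky roller trap actor that works as a short-fuse bomb, exploding on a timer after it spawns.
; BeginPlay scales the static mesh uniformly by BompScale, waits, then spawns a fireball explosion at the mesh's location.
; AddRadialForce is called on the spawned particle component itself, so it does not push surrounding objects.
; After further short delays the mesh is destroyed, then the actor, with no overlap or tick logic.
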(event `self.ReceiveBeginPlay`
  (bind _bompscale (`self.BompScale`))
  (bind _returnvalue (`SceneComponent.K2_GetComponentLocation` (`self.StaticMesh`)))
  (`SceneComponent.SetWorldScale3D` (`self.StaticMesh`) (`KismetMathLibrary.MakeVector` _bompscale _bompscale _bompscale))
  (`KismetSystemLibrary.Delay` 3.0)
  (bind _returnvalue_2 (`GameplayStatics.SpawnEmitterAtLocation` "/Game/ExampleContent/Blueprint_Communication/Effects/P_Explosion_Fireball.P_Explosion_Fireball" _returnvalue))
  (`PrimitiveComponent.AddRadialForce` _returnvalue_2 _returnvalue 2000.0 2000.0 "RIF_Constant" false)
  (`KismetSystemLibrary.Delay` 1.0)
  (`ActorComponent.K2_DestroyComponent` (`self.StaticMesh`))
  (`KismetSystemLibrary.Delay` 1.0)
  (`self.K2_DestroyActor`))

(event `self.ReceiveTick`
  (params (DeltaSeconds :type "Float (single-precision)")))

(fn `UserConstructionScript`)